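; Enemy character that walks a looping patrol, chases the player on sight and can be killed by the player at close range.
; Tick drives AI MoveTo between patrol points with a pause at each, while PawnSensing switches to chase speed and targets the player.
; KillBox overlap shows the F component and enables a one-time kill when the player attempts it.
; Death is faked by tipping and lowering the actor, disabling movement and pausing animation.
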(event `self.ReceiveBeginPlay`
  (bind _asbp_third_person_character (cast `/Game/ThirdPerson/Blueprints/BP_ThirdPersonCharacter` (`GameplayStatics.GetPlayerCharacter` 0)))
  (set `self.PlayerRef` _asbp_third_person_character))

(event `self.ReceiveTick`
  (params (DeltaSeconds :type "Float (single-precision)"))
  (bind (_returnvalue_roll _returnvalue_pitch _returnvalue_yaw) (`KismetMathLibrary.BreakRotator` (`self.K2_GetActorRotation`)))
  (bind (_returnvalue_x _returnvalue_y _returnvalue_z) (`KismetMathLibrary.BreakVector` (`self.K2_GetActorLocation`)))
  (`|ExecutionSequence`
    (:`then_0`
      (if (`self.IsAlive`)
        (if (not (`self.MovingToTarget`))
          (set `CharacterMovementComponent.MaxWalkSpeed` (`KismetMathLibrary.Conv_IntToDouble` (`self.PatrolSpeed`)) (`self.CharacterMovement`))
          (`|AIMoveTo` self (`self.K2_GetActorLocation` (`|GetArrayItem` (`self.PatrolPoints`) (`self.CurrentPatrolIndex`))) null
            (:`then`
              (set `self.MovingToTarget` true))
            (:`OnSuccess`
              (`KismetSystemLibrary.Delay` 3.0)
              (set `self.MovingToTarget` false)
              (bind _result (`/Engine/EditorBlueprintResources/StandardMacros.IncrementInt` (`self.CurrentPatrolIndex`))
                (:`  `
                  (set `self.CurrentPatrolIndex` (mod _result (`KismetArrayLibrary.Array_Length` (`self.PatrolPoints`)))))))))
        (else
          (set `SkeletalMeshComponent.bPauseAnims` true (`self.Mesh`)))))
    (:`then_1`
      (if (and (`self.PlayerIsInKillRange`) (`/Game/ThirdPerson/Blueprints/BP_ThirdPersonCharacter.TryingToKill` (`self.PlayerRef`)))
        (`/Engine/EditorBlueprintResources/StandardMacros.DoOnce` false
          (:`Completed`
            (set `self.IsAlive` false)
            (`self.K2_SetActorRotation` (`KismetMathLibrary.MakeRotator` (+ _returnvalue_roll 90.0) _returnvalue_pitch _returnvalue_yaw))
            (`self.K2_SetActorLocation` (`KismetMathLibrary.MakeVector` _returnvalue_x _returnvalue_y (- _returnvalue_z 50.0)))
            (`CharacterMovementComponent.DisableMovement` (`self.CharacterMovement`))
            (`ActorComponent.K2_DestroyComponent` (`self.KillBox`))))))))

(event `self.PawnSensing.OnSeePawn`
  (params (Pawn :type "Pawn Object Reference"))
  (`|ExecutionSequence`
    (:`then_0`
      (if (`self.ActorHasTag` Pawn "Player")
        (set `CharacterMovementComponent.MaxWalkSpeed` (`KismetMathLibrary.Conv_IntToDouble` (`self.ChaseSpeed`)) (`self.CharacterMovement`))
        (`|AIMoveTo` self (0.0 0.0 0.0) (`self.PlayerRef`))))))

(event `self.KillBox.OnComponentBeginOverlap`
  (params (OverlappedComponent :type "PrimitiveComponent Object Reference") (OtherActor :type "Actor Object Reference") (OtherComp :type "PrimitiveComponent Object Reference") (OtherBodyIndex :type Integer) (bFromSweep :type Boolean) (SweepResult :type "HitResult Structure (by ref)"))
  (if (`self.ActorHasTag` OtherActor "Player")
    (set `self.PlayerIsInKillRange` true)
    (`SceneComponent.SetHiddenInGame` (`self.F`) false false)))

(event `self.KillBox.OnComponentEndOverlap`
  (params (OverlappedComponent :type "PrimitiveComponent Object Reference") (OtherActor :type "Actor Object Reference") (OtherComp :type "PrimitiveComponent Object Reference") (OtherBodyIndex :type Integer))
  (if (`self.ActorHasTag` OtherActor "Player")
    (set `self.PlayerIsInKillRange` false)
    (`SceneComponent.SetHiddenInGame` (`self.F`) true false)))

(fn `UserConstructionScript`)