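; BP_Kendrick is an AI-moved pawn that walks through an array of patrol point actors in order.
; On Tick, when both movement flags allow it, it issues AI MoveTo toward the current point and clears CanMoveToTarget so the request is not repeated.
; Success restores the flag and increments the patrol index, which never wraps in this graph; a failed move leaves the flag cleared.
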(event `self.ReceiveTick`
  (params (DeltaSeconds :type "Float (single-precision)"))
  (if (and (`self.CanMoveToTarget`) (`self.CanMove`))
    (`|AIMoveTo` self (`self.K2_GetActorLocation` (`|GetArrayItem` (`self.PatrolPoints`) (`self.CurrentPatrolIndex`))) null
      (:`then`
        (set `self.CanMoveToTarget` false))
      (:`OnSuccess`
        (set `self.CanMoveToTarget` true)
        (`/Engine/EditorBlueprintResources/StandardMacros.IncrementInt` (`self.CurrentPatrolIndex`))))))

(fn `UserConstructionScript`)