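; Sentry turret actor that turns to track the player character.
; BeginPlay caches the third-person player character.
; Each Tick yaws Cylinder1 toward the player's mesh, using the normalized direction from Cube1 and discarding pitch and roll.
; Tick also compares that distance against MaxFireDistance, but the branch is empty, so no firing is implemented.
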(event `self.ReceiveBeginPlay`
  (bind _asbp_third_person_character (cast `/Game/ThirdPerson/Blueprints/BP_ThirdPersonCharacter` (`GameplayStatics.GetPlayerCharacter` 0)))
  (set `self.PlayerRef` _asbp_third_person_character))

(event `self.ReceiveTick`
  (params (DeltaSeconds :type "Float (single-precision)"))
  (bind _returnvalue (- (`SceneComponent.K2_GetComponentLocation` (`Character.Mesh` (`self.PlayerRef`))) (`SceneComponent.K2_GetComponentLocation` (`self.Cube1`))))
  (`SceneComponent.K2_SetWorldRotation` (`self.Cylinder1`) (`KismetMathLibrary.MakeRotator` 0.0 0.0 (.yaw (`KismetMathLibrary.MakeRotationFromAxes` (`KismetMathLibrary.Normal` _returnvalue)))) false false)
  (if (>= (`self.MaxFireDistance`) (`KismetMathLibrary.VSize` _returnvalue))
    _))

(fn `UserConstructionScript`)