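; BP_Gun1 is a weapon pickup that the player collects by interacting with it.
; Its Box overlap events show or hide a collect prompt for actors tagged Player.
; On interaction it destroys itself, sets GunCollected on the character, unhides that character's Gun and calls SetAmmoUI on the Canvas of the player controller cached at BeginPlay.
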(event `self.ReceiveBeginPlay`
  (bind _asbp_player_controller (cast `/Game/ThirdPerson/Blueprints/BP_PlayerController` (`GameplayStatics.GetPlayerController` 0)))
  (set `self.PlayerController` _asbp_player_controller))

(event `/Game/Blueprints/Interfaces/BPI_Interactions.OnInteraction`
  (params (CharacterReference :type "/Game/ThirdPerson/Blueprints/BP_ThirdPersonCharacter Object Reference"))
  (`self.K2_DestroyActor`)
  (set `/Game/ThirdPerson/Blueprints/BP_ThirdPersonCharacter.GunCollected` true CharacterReference)
  (`SceneComponent.SetHiddenInGame` (`/Game/ThirdPerson/Blueprints/BP_ThirdPersonCharacter.Gun` CharacterReference) false false)
  (`/Game/Blueprints/UI/WBP_Canvas.SetAmmoUI` (`/Game/ThirdPerson/Blueprints/BP_PlayerController.Canvas` (`self.PlayerController`))))

(event `self.Box.OnComponentBeginOverlap`
  (params (OverlappedComponent :type "PrimitiveComponent Object Reference") (OtherActor :type "Actor Object Reference") (OtherComp :type "PrimitiveComponent Object Reference") (OtherBodyIndex :type Integer) (bFromSweep :type Boolean) (SweepResult :type "HitResult Structure (by ref)"))
  (if (`self.ActorHasTag` OtherActor "Player")
    (`SceneComponent.SetHiddenInGame` (`self.CollectPrompt`) false false)))

(event `self.Box.OnComponentEndOverlap`
  (params (OverlappedComponent :type "PrimitiveComponent Object Reference") (OtherActor :type "Actor Object Reference") (OtherComp :type "PrimitiveComponent Object Reference") (OtherBodyIndex :type Integer))
  (if (`self.ActorHasTag` OtherActor "Player")
    (`SceneComponent.SetHiddenInGame` (`self.CollectPrompt`) true false)))

(fn `UserConstructionScript`)