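; BP_Gun is a weapon Blueprint that fires a debug-drawn hitscan trace from its barrel.
; OnShoot checks the passed character's AmmoCount, traces on Visibility, then decrements and prints the cached player's count, leaving the hit unused.
; An uncalled Reloading function attempts a magazine refill from a stash.
; Its guard requires an overfilled magazine, and it sets the magazine before computing the stash deduction.
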(event `self.ReceiveBeginPlay`
  (bind _asbp_third_person_character (cast `/Game/ThirdPerson/Blueprints/BP_ThirdPersonCharacter` (`GameplayStatics.GetPlayerCharacter` 0)))
  (set `self.PlayerRef` _asbp_third_person_character))

(event `/Game/Blueprints/Interfaces/BPI_Fire.OnShoot`
  (params (CharacterRef :type "/Game/ThirdPerson/Blueprints/BP_ThirdPersonCharacter Object Reference"))
  (bind _gunbarrel (`self.GunBarrel`))
  (bind _returnvalue (`SceneComponent.K2_GetComponentLocation` _gunbarrel))
  (if (> (`/Game/ThirdPerson/Blueprints/BP_ThirdPersonCharacter.AmmoCount` CharacterRef) 0)
    (bind _outhit (`KismetSystemLibrary.LineTraceSingle` :`Start` _returnvalue :`End` (+ _returnvalue (* (`self.FireRange`) (`KismetMathLibrary.GetForwardVector` (`SceneComponent.K2_GetComponentRotation` _gunbarrel)))) :`TraceChannel` "TraceTypeQuery1" :`DrawDebugType` "ForDuration"))
    (bind _result (`/Engine/EditorBlueprintResources/StandardMacros.DecrementInt` (`/Game/ThirdPerson/Blueprints/BP_ThirdPersonCharacter.AmmoCount` (`self.PlayerRef`)))
      (:`  `
        (`KismetSystemLibrary.PrintString` (`KismetStringLibrary.Conv_IntToString` _result))))))

(fn `Reloading`
  (params (CurrentAmmoMagazine :type Integer) (CurrentAmmoStash :type Integer) (MaxAmmoMagazine :type Integer) (IsReloading :type Boolean))
  (if (and (> CurrentAmmoMagazine MaxAmmoMagazine) (> CurrentAmmoStash 0))
    (set `self.IsReloading` true)
    (if (>= (+ (`self.CurrentAmmoMagazine`) (`self.CurrentAmmoStash`)) (`self.MaxAmmoMagazine`))
      (set `self.CurrentAmmoMagazine` (`self.MaxAmmoMagazine`))
      (set `self.CurrentAmmoStash` (- (`self.CurrentAmmoStash`) (- (`self.MaxAmmoMagazine`) (`self.CurrentAmmoMagazine`))))
      (set `self.IsReloading` false)
      (return)
      (else
        (set `self.CurrentAmmoMagazine` (+ (`self.CurrentAmmoMagazine`) (`self.CurrentAmmoStash`)))
        (set `self.CurrentAmmoStash` 0)
        (set `self.IsReloading` false)
        (return)))
    (else
      (return))))

(fn `UserConstructionScript`)