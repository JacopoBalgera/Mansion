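; Enemy shooter AI that turns to face the player each Tick and alternates between crouching and standing to fire.
; After a BeginPlay opening volley, crouch and stand events call each other in a randomly timed loop gated by IsAlive.
; Shots are debug-drawn line traces with random aim offset, calling the player's Death on hitting a "Player"-tagged actor.
; EnemyDeath ragdolls the mesh with a camera-forward impulse and hides the gun.
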(event `self.ReceiveBeginPlay`
  (bind _returnvalue (`KismetMathLibrary.RandomFloatInRange` 0.2 0.4))
  ; BeginPlay
  (`|ExecutionSequence`
    (:`then_0`
      (bind _asbp_third_person_character (cast `/Game/ThirdPerson/Blueprints/BP_ThirdPersonCharacter` (`GameplayStatics.GetPlayerCharacter` 0)))
      (set `self.PlayerRef` _asbp_third_person_character))
    (:`then_1`
      (`KismetSystemLibrary.Delay` 4.6)
      (`self.EnemyShooting`)
      (`KismetSystemLibrary.Delay` _returnvalue)
      (`self.EnemyShooting`)
      (`KismetSystemLibrary.Delay` _returnvalue)
      (`self.EnemyShooting`)
      (`KismetSystemLibrary.Delay` 2.5)
      (`self.EnemyCrouch`))))

(event `self.ReceiveTick`
  (params (DeltaSeconds :type "Float (single-precision)"))
  (bind (_returnvalue_roll _returnvalue_pitch _returnvalue_yaw) (`KismetMathLibrary.BreakRotator` (`KismetMathLibrary.FindLookAtRotation` (`self.K2_GetActorLocation`) (`self.K2_GetActorLocation` (`self.PlayerRef`)))))
  ; EnemyRotation
  (`self.K2_SetActorRotation` (`KismetMathLibrary.MakeRotator` 0.0 0.0 _returnvalue_yaw)))

(event `EnemyDeath`
  (bind _mesh (`self.Mesh`))
  ; EnemyDeath
  (`|ExecutionSequence`
    (:`then_0`
      (`PrimitiveComponent.SetSimulatePhysics` _mesh true)
      (`PrimitiveComponent.SetCollisionEnabled` (`self.CapsuleComponent`) "PhysicsOnly")
      (`PrimitiveComponent.SetCollisionEnabled` _mesh "PhysicsOnly")
      (`PrimitiveComponent.AddImpulse` _mesh (10.0 10.0 10.0) "None" false)
      (`PrimitiveComponent.AddImpulse` _mesh (* (`KismetMathLibrary.GetForwardVector` (`SceneComponent.K2_GetComponentRotation` (`/Game/ThirdPerson/Blueprints/BP_ThirdPersonCharacter.FollowCamera` (`self.PlayerRef`)))) 1500.0) "None" true)
      (`SceneComponent.SetHiddenInGame` (`self.Gun`) true false))
    (:`then_1`
      (set `self.IsAlive` false))))

(event `EnemyCrouch`
  ; EnemyCrouch
  (if (`self.IsAlive`)
    (`|ExecutionSequence`
      (:`then_0`
        (`self.Crouch`))
      (:`then_1`
        (`SkeletalMeshComponent.SetAnimation` (`self.Mesh`) "/Game/Crouch_Idle_Rifle_Ironsights.Crouch_Idle_Rifle_Ironsights"))
      (:`then_2`
        (`KismetSystemLibrary.Delay` (`KismetMathLibrary.RandomFloatInRange` 3.5 4.5))
        (`self.EnemyStanding`)))))

(event `EnemyStanding`
  (bind _returnvalue (`KismetMathLibrary.RandomFloatInRange` 0.8 1.6))
  ; EnemyStanding
  (if (`self.IsAlive`)
    (`|ExecutionSequence`
      (:`then_0`
        (`self.UnCrouch`))
      (:`then_1`
        (`SkeletalMeshComponent.SetAnimation` (`self.Mesh`) "/Game/AnimStarterPack/Animations/Idle_Pistol.Idle_Pistol"))
      (:`then_2`
        (if (`self.IsAlive`)
          (`KismetSystemLibrary.Delay` (`KismetMathLibrary.RandomFloatInRange` 1.5 2.7))
          (`self.EnemyShooting`)
          (`KismetSystemLibrary.Delay` _returnvalue)
          (if (`self.IsAlive`)
            (`self.EnemyShooting`)
            (`KismetSystemLibrary.Delay` _returnvalue)
            (if (`self.IsAlive`)
              (`self.EnemyShooting`)
              (`KismetSystemLibrary.Delay` 1.5)
              (`self.EnemyCrouch`))))))))

(event `EnemyShooting`
  (bind _returnvalue (`KismetMathLibrary.RandomFloatInRange` 0.0 70.0))
  ; EnemyShooting
  (bind (_outhit _returnvalue_2) (`KismetSystemLibrary.LineTraceSingle` :`Start` (`SceneComponent.K2_GetComponentLocation` (`self.Gun`)) :`End` (+ (`SceneComponent.K2_GetComponentLocation` (`Actor.RootComponent` (`self.PlayerRef`))) (`KismetMathLibrary.MakeVector` _returnvalue _returnvalue _returnvalue)) :`TraceChannel` "TraceTypeQuery1" :`bTraceComplex` true :`DrawDebugType` "ForDuration"))
  (if _returnvalue_2
    (if (`self.ActorHasTag` (`.HitActor` (`GameplayStatics.BreakHitResult` _outhit)) "Player")
      (`/Game/ThirdPerson/Blueprints/BP_ThirdPersonCharacter.Death` (`self.PlayerRef`)))))

(fn `UserConstructionScript`)