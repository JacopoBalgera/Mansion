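; Enemy AI controller that runs the BT_EnemyBase behavior tree and switches its blackboard state between Patrol, Chase and Dead.
; Perception updates are filtered for successful sight stimuli; spotting a Player-tagged actor while patrolling stores it as the target and starts Chase.
; A forgotten target returns the state to Patrol.
; SetStateAsDead writes the Dead state but has no caller within this Blueprint.
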(event `self.ReceivePossess`
  (params (PossessedPawn :type "Pawn Object Reference"))
  (`self.RunBehaviorTree` "/Game/Blueprints/AI/BT_EnemyBase.BT_EnemyBase")
  (`self.SetStateAsPatrol`))

(event `self.AIPerception.OnPerceptionUpdated`
  (params (UpdatedActors :type "Array of Actor Object Reference (by ref)"))
  (for _array_element UpdatedActors
    (bind _sensed (`self.CanSenseActor` _array_element "NewEnumerator1"))
    (if _sensed
      (`self.HandleSensedSight` _array_element))))

(event `self.AIPerception.OnTargetPerceptionForgotten`
  (params (Actor :type "Actor Object Reference"))
  (`self.SetStateAsPatrol`))

(fn `CanSenseActor`
  (params (Actor :type "Actor Object Reference") (Sense :type "/Game/Blueprints/AI/Enums/E_AISense Enum" :default "NewEnumerator0"))
  (returns (Sensed :type Boolean) (`Array Element` :type "AIStimulus Structure"))
  (bind _info (`AIPerceptionComponent.GetActorsPerception` (`self.AIPerception`) Actor))
  (for _array_element (`.LastSensedStimuli` (break `ActorPerceptionBlueprintInfo` _info))
    (bind _returnvalue (`AIPerceptionSystem.GetSenseClassForStimulus` _array_element))
    (if (== _returnvalue (select `/Game/Blueprints/AI/Enums/E_AISense` Sense :`NewEnumerator1` "/Script/AIModule.AISense_Sight" :`NewEnumerator2` "/Script/AIModule.AISense_Hearing" :!type "Object Class Reference"))
      (return (`.bSuccessfullySensed` (break `AIStimulus` _array_element)) _array_element))))

(fn `GetCurrentState`
  (returns (State :type "/Game/Blueprints/AI/Enums/E_AIState Enum"))
  (return (cast `/Game/Blueprints/AI/Enums/E_AIState` (`BlackboardComponent.GetValueAsEnum` (`self.Blackboard`) (`self.EnemyStateKeyName`)))))

(fn `HandleSensedSight`
  (params (Actor :type "Actor Object Reference"))
  (bind _state (`self.GetCurrentState`))
  (switch `/Game/Blueprints/AI/Enums/E_AIState` _state
    (:`NewEnumerator0`
      (if (`self.ActorHasTag` Actor "Player")
        (`self.SetStateAsChase` Actor)))))

(fn `SetStateAsChase`
  (params (ChaseTarget :type "Actor Object Reference"))
  (`BlackboardComponent.SetValueAsObject` (`self.Blackboard`) (`self.GetToPlayerKeyName`) ChaseTarget)
  (`BlackboardComponent.SetValueAsEnum` (`self.Blackboard`) (`self.EnemyStateKeyName`) (enumliteral `/Game/Blueprints/AI/Enums/E_AIState` "NewEnumerator1")))

(fn `SetStateAsDead`
  (`BlackboardComponent.SetValueAsEnum` (`self.Blackboard`) (`self.EnemyStateKeyName`) (enumliteral `/Game/Blueprints/AI/Enums/E_AIState` "NewEnumerator2")))

(fn `SetStateAsPatrol`
  (`BlackboardComponent.SetValueAsEnum` (`self.Blackboard`) (`self.EnemyStateKeyName`) (enumliteral `/Game/Blueprints/AI/Enums/E_AIState` "NewEnumerator0")))

(fn `UserConstructionScript`)