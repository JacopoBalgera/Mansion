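; Base AI enemy character that the player can kill from within a KillBox overlap, and that kills the player on DeathBox contact while alive.
; KillBox toggles the killable flag and the F component's visibility, and Death, presumably bound to the player's kill event, checks that flag.
; Death ragdolls the mesh along the camera's forward vector, disables capsule collision and stops the AI brain.
; It also exposes its patrol route and speed presets.
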(event `self.ReceiveBeginPlay`
  ; BeginPlay
  (bind _asbp_enemy_aicontroller (cast `/Game/Blueprints/AI/BP_EnemyAIController` (`AIBlueprintHelperLibrary.GetAIController` self)))
  (set `self.AIControllerRef` _asbp_enemy_aicontroller)
  (bind _asbp_third_person_character (cast `/Game/ThirdPerson/Blueprints/BP_ThirdPersonCharacter` (`GameplayStatics.GetPlayerCharacter` 0)))
  (bind _output_get (set `self.PlayerRef` _asbp_third_person_character))
  (add `/Game/ThirdPerson/Blueprints/BP_ThirdPersonCharacter.KillEvent` _output_get (`|CreateDelegate` :!event `Death`)))

(event `self.KillBox.OnComponentBeginOverlap`
  (params (OverlappedComponent :type "PrimitiveComponent Object Reference") (OtherActor :type "Actor Object Reference") (OtherComp :type "PrimitiveComponent Object Reference") (OtherBodyIndex :type Integer) (bFromSweep :type Boolean) (SweepResult :type "HitResult Structure (by ref)"))
  ; KillBoxCheck
  (if (and (`self.ActorHasTag` OtherActor "Player") (`self.IsAlive`))
    (set `self.IsKillable` true)
    (`SceneComponent.SetHiddenInGame` (`self.F`) false false)))

(event `self.KillBox.OnComponentEndOverlap`
  (params (OverlappedComponent :type "PrimitiveComponent Object Reference") (OtherActor :type "Actor Object Reference") (OtherComp :type "PrimitiveComponent Object Reference") (OtherBodyIndex :type Integer))
  ; KillBoxCheck
  (if (`self.ActorHasTag` OtherActor "Player")
    (set `self.IsKillable` false)
    (`SceneComponent.SetHiddenInGame` (`self.F`) true false)))

(event `Death`
  (bind _mesh (`self.Mesh`))
  (bind _aicontrollerref (`self.AIControllerRef`))
  ; DeathLogic
  (if (`self.IsKillable`)
    (`|ExecutionSequence`
      (:`then_0`
        (`PrimitiveComponent.SetSimulatePhysics` _mesh true)
        (`PrimitiveComponent.SetCollisionEnabled` _mesh "PhysicsOnly")
        (`PrimitiveComponent.AddImpulse` _mesh (10.0 10.0 10.0) "None" false)
        (`PrimitiveComponent.AddImpulse` _mesh (* (`KismetMathLibrary.GetForwardVector` (`SceneComponent.K2_GetComponentRotation` (`/Game/ThirdPerson/Blueprints/BP_ThirdPersonCharacter.FollowCamera` (`self.PlayerRef`)))) 1500.0) "None" true))
      (:`then_1`
        (`PrimitiveComponent.SetCollisionEnabled` (`self.CapsuleComponent`) "NoCollision")
        (set `self.IsAlive` false))
      (:`then_2`
        (`BrainComponent.StopLogic` (`AIController.BrainComponent` _aicontrollerref) "")
        (`/Game/Blueprints/AI/BP_EnemyAIController.SetStateAsDead` _aicontrollerref)))))

(event `self.DeathBox.OnComponentBeginOverlap`
  (params (OverlappedComponent :type "PrimitiveComponent Object Reference") (OtherActor :type "Actor Object Reference") (OtherComp :type "PrimitiveComponent Object Reference") (OtherBodyIndex :type Integer) (bFromSweep :type Boolean) (SweepResult :type "HitResult Structure (by ref)"))
  ; DeathBox
  (if (`self.ActorHasTag` OtherActor "Player")
    (if (`self.IsAlive`)
      (`/Game/ThirdPerson/Blueprints/BP_ThirdPersonCharacter.Death` (`self.PlayerRef`)))))

(fn `GetPatrolRoute`
  (returns (PatrolRoute :type "/Game/Blueprints/AI/BP_PatrolRoute Object Reference"))
  (return (`self.PatrolRoute`)))

(fn `SetMovementSpeed`
  (params (Speed :type "/Game/Blueprints/AI/Enums/E_MovementSpeed Enum" :default "NewEnumerator0"))
  (returns (SpeedValue :type "Float (double-precision)"))
  (bind _output_get (set `CharacterMovementComponent.MaxWalkSpeed` (select `/Game/Blueprints/AI/Enums/E_MovementSpeed` Speed :`NewEnumerator1` 180.0 :`NewEnumerator2` 350.0 :!type "Float (single-precision)") (`self.CharacterMovement`)))
  (return _output_get))

(fn `UserConstructionScript`)