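; Stationary AI sentry that turns its head to track the third-person player and fires projectiles when they are within range.
; Each tick it yaws the head toward the player's mesh and plays the FireRate timeline, which paces the shots.
; On timeline completion, an in-range check spawns a projectile from the nose and restarts the timer.
; Each projectile's hit event reports back, printing an Italian hit or miss message.
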(event `self.ReceiveBeginPlay`
  (bind _asbp_third_person_character (cast `/Game/ThirdPerson/Blueprints/BP_ThirdPersonCharacter` (`GameplayStatics.GetPlayerCharacter` 0)))
  (set `self.PlayerRef` _asbp_third_person_character))

(event `self.ReceiveTick`
  (params (DeltaSeconds :type "Float (single-precision)"))
  (bind _nose (`self.Nose`))
  (bind _returnvalue (`SceneComponent.K2_GetComponentRotation` _nose))
  (bind _returnvalue_2 (- (`SceneComponent.K2_GetComponentLocation` (`Character.Mesh` (`self.PlayerRef`))) (`SceneComponent.K2_GetComponentLocation` (`self.Nose`))))
  (`SceneComponent.K2_SetWorldRotation` (`self.Head`) (`KismetMathLibrary.MakeRotator` 0.0 0.0 (.yaw (`KismetMathLibrary.MakeRotationFromAxes` (`KismetMathLibrary.Normal` _returnvalue_2)))) false false)
  (`Timeline|FireRate` :!label _label
    (:`Finished`
      (if (>= (`self.MaxFireDistance`) (`KismetMathLibrary.VSize` _returnvalue_2))
        (`|ExecutionSequence`
          (:`then_0`
            (bind _returnvalue_3 (`|SpawnActorFromClass` "/Game/FirstPerson/Blueprints/BP_FirstPersonProjectile.BP_FirstPersonProjectile_C" (`KismetMathLibrary.MakeTransform` (+ (`SceneComponent.K2_GetComponentLocation` _nose) (`KismetMathLibrary.GreaterGreater_VectorRotator` (`self.ProjectileOffset`) _returnvalue)) _returnvalue) "Undefined" "MultiplyWithRoot" null null))
            (add `/Game/FirstPerson/Blueprints/BP_FirstPersonProjectile.ProjectileHit` _returnvalue_3 (delegate `Hit`)))
          (:`then_1`
            (goto _label :!via `PlayFromStart`)))))))

(event `Hit`
  (params (`Hit Variable` :type "HitResult Structure"))
  (cast `/Game/ThirdPerson/Blueprints/BP_ThirdPersonCharacter` (`.HitActor` (`GameplayStatics.BreakHitResult` `Hit Variable`))
    (:`then`
      (`KismetSystemLibrary.PrintString` "Colpito"))
    (:`CastFailed`
      (`KismetSystemLibrary.PrintString` "Mancato"))))

(fn `UserConstructionScript`)