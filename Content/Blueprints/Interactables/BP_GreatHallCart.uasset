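; BP_GreatHallCart is an interactable cart that the player can attach to themselves and carry along, then release.
; An overlap box shows or hides a text render while the player is inside it.
; Each interaction flips between attaching the cart to the player and detaching it, keeping world transforms.
; The same toggle swaps Enhanced Input mapping contexts between the default and carrying sets.
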(event `self.ReceiveBeginPlay`
  ; BeginPlay
  (`|ExecutionSequence`
    (:`then_0`
      (bind _asbp_third_person_character (cast `/Game/ThirdPerson/Blueprints/BP_ThirdPersonCharacter` (`GameplayStatics.GetPlayerCharacter` 0)))
      (set `self.PlayerRef` _asbp_third_person_character))
    (:`then_1`
      (bind _asbp_player_controller (cast `/Game/ThirdPerson/Blueprints/BP_PlayerController` (`GameplayStatics.GetPlayerController` 0)))
      (set `self.ControllerRef` _asbp_player_controller))))

(event `self.TextBox.OnComponentBeginOverlap`
  (params (OverlappedComponent :type "PrimitiveComponent Object Reference") (OtherActor :type "Actor Object Reference") (OtherComp :type "PrimitiveComponent Object Reference") (OtherBodyIndex :type Integer) (bFromSweep :type Boolean) (SweepResult :type "HitResult Structure (by ref)"))
  ; Text
  (if (== OtherActor (`self.PlayerRef`))
    (`SceneComponent.SetHiddenInGame` (`self.TextRender`) false false)))

(event `self.TextBox.OnComponentEndOverlap`
  (params (OverlappedComponent :type "PrimitiveComponent Object Reference") (OtherActor :type "Actor Object Reference") (OtherComp :type "PrimitiveComponent Object Reference") (OtherBodyIndex :type Integer))
  ; Text
  (if (== OtherActor (`self.PlayerRef`))
    (`SceneComponent.SetHiddenInGame` (`self.TextRender`) true false)))

(event `/Game/Blueprints/Interfaces/BPI_Interactions.OnInteraction`
  (params (CharacterReference :type "/Game/ThirdPerson/Blueprints/BP_ThirdPersonCharacter Object Reference"))
  (bind _returnvalue (pcsubsystem `EnhancedInputLocalPlayerSubsystem` (`self.ControllerRef`)))
  (bind _returnvalue_2 (pcsubsystem `EnhancedInputLocalPlayerSubsystem` (`self.ControllerRef`)))
  ; AttachToPlayer
  (`/Engine/EditorBlueprintResources/StandardMacros.FlipFlop`
    (:`A`
      (`self.K2_AttachToActor` (`self.PlayerRef`) "None" "KeepWorld" "KeepWorld" "KeepWorld" false)
      (`EnhancedInputSubsystemInterface.RemoveMappingContext` _returnvalue_2 "/Game/ThirdPerson/Input/IMC_Default.IMC_Default" (struct))
      (`EnhancedInputSubsystemInterface.AddMappingContext` _returnvalue_2 "/Game/ThirdPerson/Input/IMC_DefaultCarrying.IMC_DefaultCarrying" 0 (struct)))
    (:`B`
      (`self.K2_DetachFromActor` "KeepWorld" "KeepWorld" "KeepWorld")
      (`EnhancedInputSubsystemInterface.RemoveMappingContext` _returnvalue "/Game/ThirdPerson/Input/IMC_DefaultCarrying.IMC_DefaultCarrying" (struct))
      (`EnhancedInputSubsystemInterface.AddMappingContext` _returnvalue "/Game/ThirdPerson/Input/IMC_Default.IMC_Default" 0 (struct)))))

(fn `UserConstructionScript`)