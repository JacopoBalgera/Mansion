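; BP_Safe is an interactable safe with a keypad code UI and a swinging door.
; OnInteraction reveals the keypad widgets on the controller's Canvas via render opacity and swaps input mapping from IMC_Default to IMC_UI.
; SafeOpening rotates the door's yaw with a timeline; code checking and its live trigger are not in this graph.
; Player-tagged box overlaps unhide the interaction prompt on both begin and end, so it never re-hides here.
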(event `/Game/Blueprints/Interfaces/BPI_Interactions.OnInteraction`
  (params (CharacterReference :type "/Game/ThirdPerson/Blueprints/BP_ThirdPersonCharacter Object Reference"))
  (bind _controllerref (`/Game/ThirdPerson/Blueprints/BP_ThirdPersonCharacter.ControllerRef` CharacterReference))
  (bind _returnvalue (pcsubsystem `EnhancedInputLocalPlayerSubsystem` _controllerref))
  ; OnInteraction
  (`Widget.SetRenderOpacity` (`/Game/Blueprints/UI/WBP_Canvas.Button0` (`/Game/ThirdPerson/Blueprints/BP_PlayerController.Canvas` _controllerref)) 1.0)
  (`Widget.SetRenderOpacity` (`/Game/Blueprints/UI/WBP_Canvas.Button1` (`/Game/ThirdPerson/Blueprints/BP_PlayerController.Canvas` _controllerref)) 1.0)
  (`Widget.SetRenderOpacity` (`/Game/Blueprints/UI/WBP_Canvas.Button2` (`/Game/ThirdPerson/Blueprints/BP_PlayerController.Canvas` _controllerref)) 1.0)
  (`Widget.SetRenderOpacity` (`/Game/Blueprints/UI/WBP_Canvas.Button3` (`/Game/ThirdPerson/Blueprints/BP_PlayerController.Canvas` _controllerref)) 1.0)
  (`Widget.SetRenderOpacity` (`/Game/Blueprints/UI/WBP_Canvas.Button4` (`/Game/ThirdPerson/Blueprints/BP_PlayerController.Canvas` _controllerref)) 1.0)
  (`Widget.SetRenderOpacity` (`/Game/Blueprints/UI/WBP_Canvas.Button5` (`/Game/ThirdPerson/Blueprints/BP_PlayerController.Canvas` _controllerref)) 1.0)
  (`Widget.SetRenderOpacity` (`/Game/Blueprints/UI/WBP_Canvas.Button6` (`/Game/ThirdPerson/Blueprints/BP_PlayerController.Canvas` _controllerref)) 1.0)
  (`Widget.SetRenderOpacity` (`/Game/Blueprints/UI/WBP_Canvas.Button7` (`/Game/ThirdPerson/Blueprints/BP_PlayerController.Canvas` _controllerref)) 1.0)
  (`Widget.SetRenderOpacity` (`/Game/Blueprints/UI/WBP_Canvas.Button8` (`/Game/ThirdPerson/Blueprints/BP_PlayerController.Canvas` _controllerref)) 1.0)
  (`Widget.SetRenderOpacity` (`/Game/Blueprints/UI/WBP_Canvas.Button9` (`/Game/ThirdPerson/Blueprints/BP_PlayerController.Canvas` _controllerref)) 1.0)
  (`Widget.SetRenderOpacity` (`/Game/Blueprints/UI/WBP_Canvas.ButtonBack` (`/Game/ThirdPerson/Blueprints/BP_PlayerController.Canvas` _controllerref)) 1.0)
  (`Widget.SetRenderOpacity` (`/Game/Blueprints/UI/WBP_Canvas.ButtonEnter` (`/Game/ThirdPerson/Blueprints/BP_PlayerController.Canvas` _controllerref)) 1.0)
  (`Widget.SetRenderOpacity` (`/Game/Blueprints/UI/WBP_Canvas.CodePanel` (`/Game/ThirdPerson/Blueprints/BP_PlayerController.Canvas` _controllerref)) 1.0)
  (`Widget.SetRenderOpacity` (`/Game/Blueprints/UI/WBP_Canvas.SafePanel` (`/Game/ThirdPerson/Blueprints/BP_PlayerController.Canvas` _controllerref)) 1.0)
  (`Widget.SetRenderOpacity` (`/Game/Blueprints/UI/WBP_Canvas.Code` (`/Game/ThirdPerson/Blueprints/BP_PlayerController.Canvas` _controllerref)) 1.0)
  (`Widget.SetRenderOpacity` (`/Game/Blueprints/UI/WBP_Canvas.CloseText` (`/Game/ThirdPerson/Blueprints/BP_PlayerController.Canvas` _controllerref)) 1.0)
  (message `EnhancedInputSubsystemInterface.RemoveMappingContext` _returnvalue "/Game/ThirdPerson/Input/IMC_Default.IMC_Default" (struct))
  (message `EnhancedInputSubsystemInterface.AddMappingContext` _returnvalue "/Game/ThirdPerson/Input/IMC_UI.IMC_UI" 0 (struct)))

(event `SafeOpening`
  ; SafeOpening
  (bind (_direction _newtrack_0) (`Timeline|SafeDoorRotation`)
    (:`Update`
      (`SceneComponent.K2_SetRelativeRotation` (`self.SafeDoor`) (`KismetMathLibrary.MakeRotator` 0.0 0.0 _newtrack_0) false false))))

(event `self.Box.OnComponentBeginOverlap`
  (params (OverlappedComponent :type "PrimitiveComponent Object Reference") (OtherActor :type "Actor Object Reference") (OtherComp :type "PrimitiveComponent Object Reference") (OtherBodyIndex :type Integer) (bFromSweep :type Boolean) (SweepResult :type "HitResult Structure (by ref)"))
  ; PromptText
  (if (`self.ActorHasTag` OtherActor "Player")
    (`SceneComponent.SetHiddenInGame` (`self.InteractionPrompt`) false false)))

(event `self.Box.OnComponentEndOverlap`
  (params (OverlappedComponent :type "PrimitiveComponent Object Reference") (OtherActor :type "Actor Object Reference") (OtherComp :type "PrimitiveComponent Object Reference") (OtherBodyIndex :type Integer))
  ; PromptText
  (if (`self.ActorHasTag` OtherActor "Player")
    (`SceneComponent.SetHiddenInGame` (`self.InteractionPrompt`) false false)))

(fn `UserConstructionScript`)