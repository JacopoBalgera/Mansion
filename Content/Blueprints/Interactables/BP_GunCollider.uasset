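; BP_GunCollider is a blocking trigger that shows the player a hint about the gun.
; On BeginPlay it caches the third-person player character and the player controller.
; When the player hits its Box component without having collected the gun, it plays the TextFadeGunHint animation on the controller's Canvas widget.
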(event `self.ReceiveBeginPlay`
  (bind _asbp_third_person_character (cast `/Game/ThirdPerson/Blueprints/BP_ThirdPersonCharacter` (`GameplayStatics.GetPlayerCharacter` 0)))
  (set `self.PlayerRef` _asbp_third_person_character)
  (bind _asbp_player_controller (cast `/Game/ThirdPerson/Blueprints/BP_PlayerController` (`GameplayStatics.GetPlayerController` 0)))
  (set `self.ControllerRef` _asbp_player_controller))

(event `self.Box.OnComponentHit`
  (params (HitComponent :type "PrimitiveComponent Object Reference") (OtherActor :type "Actor Object Reference") (OtherComp :type "PrimitiveComponent Object Reference") (NormalImpulse :type "Vector Structure") (Hit :type "HitResult Structure (by ref)"))
  (bind _playerref (`self.PlayerRef`))
  (bind _canvas (`/Game/ThirdPerson/Blueprints/BP_PlayerController.Canvas` (`self.ControllerRef`)))
  (if (== OtherActor _playerref)
    (if (not (`/Game/ThirdPerson/Blueprints/BP_ThirdPersonCharacter.GunCollected` _playerref))
      (`UserWidget.PlayAnimation` _canvas (`/Game/Blueprints/UI/WBP_Canvas.TextFadeGunHint` _canvas) 0.0 1 "Forward" 1.0 false))))

(fn `UserConstructionScript`)