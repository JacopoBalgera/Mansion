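; Box trigger that, when the player enters, spawns three BP_EnemyShooter actors at preset spawn points and stages a cutscene transition.
; It removes the input mapping, drives a timeline fade on the controller's canvas, calls the GH cutscene, clears the fade and restores input after a delay.
; After a delay, it also crouches the character and shortens the camera boom.
; Any end overlap destroys the trigger after a delay.
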(event `self.Box.OnComponentBeginOverlap`
  (params (OverlappedComponent :type "PrimitiveComponent Object Reference") (OtherActor :type "Actor Object Reference") (OtherComp :type "PrimitiveComponent Object Reference") (OtherBodyIndex :type Integer) (bFromSweep :type Boolean) (SweepResult :type "HitResult Structure (by ref)"))
  (bind _returnvalue (`GameplayStatics.GetPlayerCharacter` 0))
  (if (== OtherActor _returnvalue)
    (`|ExecutionSequence`
      (:`then_0`
        (`|SpawnActorFromClass` "/Game/Blueprints/AI/BP_EnemyShooter.BP_EnemyShooter_C" (`self.SpawnPoint1`) "Undefined" "MultiplyWithRoot" null null))
      (:`then_1`
        (`|SpawnActorFromClass` "/Game/Blueprints/AI/BP_EnemyShooter.BP_EnemyShooter_C" (`self.SpawnPoint2`) "Undefined" "MultiplyWithRoot" null null))
      (:`then_2`
        (`|SpawnActorFromClass` "/Game/Blueprints/AI/BP_EnemyShooter.BP_EnemyShooter_C" (`self.SpawnPoint3`) "Undefined" "MultiplyWithRoot" null null))
      (:`then_3`
        (bind _asbp_player_controller (cast `/Game/ThirdPerson/Blueprints/BP_PlayerController` (`GameplayStatics.GetPlayerController` 0)))
        (bind _returnvalue_2 (pcsubsystem `EnhancedInputLocalPlayerSubsystem` _asbp_player_controller))
        (`EnhancedInputSubsystemInterface.RemoveMappingContext` _returnvalue_2 "/Game/ThirdPerson/Input/IMC_Default.IMC_Default" (struct))
        (bind (_direction _newtrack_0) (`Timeline|Timeline_0`)
          (:`Update`
            (bind _cutscenefade (`/Game/Blueprints/UI/WBP_Canvas.CutsceneFade` (`/Game/ThirdPerson/Blueprints/BP_PlayerController.Canvas` _asbp_player_controller)))
            (set `Widget.RenderOpacity` _newtrack_0 _cutscenefade))
          (:`Finished`
            (`self.PlayGHCutscene`)
            (set `Widget.RenderOpacity` 0.0 _cutscenefade)
            (`KismetSystemLibrary.Delay` 1.2)
            (`EnhancedInputSubsystemInterface.AddMappingContext` _returnvalue_2 "/Game/ThirdPerson/Input/IMC_Default.IMC_Default" 0 (struct)))))
      (:`then_4`
        (bind _asbp_third_person_character (cast `/Game/ThirdPerson/Blueprints/BP_ThirdPersonCharacter` _returnvalue))
        (`KismetSystemLibrary.Delay` 1.0)
        (`Character.Crouch` _asbp_third_person_character)
        (set `/Game/ThirdPerson/Blueprints/BP_ThirdPersonCharacter.IsStanding` false _asbp_third_person_character)
        (bind (_direction_2 _newtrack_0_2) (`Timeline|Timeline`)
          (:`Update`
            (set `SpringArmComponent.TargetArmLength` (`KismetMathLibrary.Lerp` 200.0 100.0 _newtrack_0_2) (`/Game/ThirdPerson/Blueprints/BP_ThirdPersonCharacter.CameraBoom` _asbp_third_person_character))))))))

(event `self.Box.OnComponentEndOverlap`
  (params (OverlappedComponent :type "PrimitiveComponent Object Reference") (OtherActor :type "Actor Object Reference") (OtherComp :type "PrimitiveComponent Object Reference") (OtherBodyIndex :type Integer))
  (`KismetSystemLibrary.Delay` 2.0)
  (`self.K2_DestroyActor`))

(fn `UserConstructionScript`)