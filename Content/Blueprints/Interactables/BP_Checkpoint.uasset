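; A one-shot checkpoint interactable that records a respawn location for the player character.
; On BeginPlay it caches player zero as a BP_ThirdPersonCharacter.
; When an actor tagged Player overlaps the Checkpoint component, it writes the root's world location to that cached character's LastCheckpointLocation, then destroys itself after a short delay.
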(event `self.ReceiveBeginPlay`
  (bind _asbp_third_person_character (cast `/Game/ThirdPerson/Blueprints/BP_ThirdPersonCharacter` (`GameplayStatics.GetPlayerCharacter` 0)))
  (set `self.PlayerRef` _asbp_third_person_character))

(event `self.Checkpoint.OnComponentBeginOverlap`
  (params (OverlappedComponent :type "PrimitiveComponent Object Reference") (OtherActor :type "Actor Object Reference") (OtherComp :type "PrimitiveComponent Object Reference") (OtherBodyIndex :type Integer) (bFromSweep :type Boolean) (SweepResult :type "HitResult Structure (by ref)"))
  (if (`self.ActorHasTag` OtherActor "Player")
    (set `/Game/ThirdPerson/Blueprints/BP_ThirdPersonCharacter.LastCheckpointLocation` (`SceneComponent.K2_GetComponentLocation` (`self.DefaultSceneRoot`)) (`self.PlayerRef`))
    (`KismetSystemLibrary.Delay` 0.2)
    (`self.K2_DestroyActor`)))

(fn `UserConstructionScript`)