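; A trigger box that springs a shooter ambush when the player walks into it.
; On player overlap it spawns two BP_EnemyShooter actors at two spawn points and starts a short timer.
; The timer plays the DontLetHimPass 2D sound and the matching text fade animation on the player controller's Canvas widget.
; Any end overlap destroys the box, with no check on which actor left.
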(event `self.Box.OnComponentBeginOverlap`
  (params (OverlappedComponent :type "PrimitiveComponent Object Reference") (OtherActor :type "Actor Object Reference") (OtherComp :type "PrimitiveComponent Object Reference") (OtherBodyIndex :type Integer) (bFromSweep :type Boolean) (SweepResult :type "HitResult Structure (by ref)"))
  (if (== OtherActor (`GameplayStatics.GetPlayerCharacter` 0))
    (`|ExecutionSequence`
      (:`then_0`
        (`|SpawnActorFromClass` "/Game/Blueprints/AI/BP_EnemyShooter.BP_EnemyShooter_C" (`self.SpawnPoint1`) "Undefined" "MultiplyWithRoot" null null))
      (:`then_1`
        (`|SpawnActorFromClass` "/Game/Blueprints/AI/BP_EnemyShooter.BP_EnemyShooter_C" (`self.SpawnPoint2`) "Undefined" "MultiplyWithRoot" null null))
      (:`then_3`
        (bind _asbp_player_controller (cast `/Game/ThirdPerson/Blueprints/BP_PlayerController` (`GameplayStatics.GetPlayerController` 0)))
        (`KismetSystemLibrary.K2_SetTimerDelegate` (delegate `CustomEvent`) 0.7)))))

(event `CustomEvent`
  (`|ExecutionSequence`
    (:`then_0`
      (`GameplayStatics.PlaySound2D` "/Game/Audios/DontLetHimPass.DontLetHimPass" 1.0 1.0 0.0 null null))
    (:`then_1`
      (bind _canvas (`/Game/ThirdPerson/Blueprints/BP_PlayerController.Canvas` (stale `self.Box.OnComponentBeginOverlap` _asbp_player_controller)))
      (`UserWidget.PlayAnimation` _canvas (`/Game/Blueprints/UI/WBP_Canvas.TextFadeDontLetHimPass` _canvas) 0.0 1 "Forward" 1.0 false))))

(event `self.Box.OnComponentEndOverlap`
  (params (OverlappedComponent :type "PrimitiveComponent Object Reference") (OtherActor :type "Actor Object Reference") (OtherComp :type "PrimitiveComponent Object Reference") (OtherBodyIndex :type Integer))
  (`ActorComponent.K2_DestroyComponent` (`self.Box`)))

(fn `UserConstructionScript`)