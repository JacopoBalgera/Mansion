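; BP_Note5 is an interactable note that shows a prompt while an actor tagged Player overlaps its box.
; On interaction it makes the note panel, close text and Note5 element on the player controller's canvas visible by setting their render opacity.
; It also swaps the Enhanced Input mapping context from default to UI.
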(event `self.OnInteraction`
  (params (CharacterReference :type "/Game/ThirdPerson/Blueprints/BP_ThirdPersonCharacter Object Reference"))
  (bind _asbp_player_controller (cast `/Game/ThirdPerson/Blueprints/BP_PlayerController` (`GameplayStatics.GetPlayerController` 0)))
  (`Widget.SetRenderOpacity` (`/Game/Blueprints/UI/WBP_Canvas.NotePanel` (`/Game/ThirdPerson/Blueprints/BP_PlayerController.Canvas` _asbp_player_controller)) 1.0)
  (`Widget.SetRenderOpacity` (`/Game/Blueprints/UI/WBP_Canvas.CloseText` (`/Game/ThirdPerson/Blueprints/BP_PlayerController.Canvas` _asbp_player_controller)) 1.0)
  (`Widget.SetRenderOpacity` (`/Game/Blueprints/UI/WBP_Canvas.Note5` (`/Game/ThirdPerson/Blueprints/BP_PlayerController.Canvas` _asbp_player_controller)) 1.0)
  (bind _returnvalue (pcsubsystem `EnhancedInputLocalPlayerSubsystem` _asbp_player_controller))
  (message `EnhancedInputSubsystemInterface.RemoveMappingContext` _returnvalue "/Game/ThirdPerson/Input/IMC_Default.IMC_Default" (struct))
  (message `EnhancedInputSubsystemInterface.AddMappingContext` _returnvalue "/Game/ThirdPerson/Input/IMC_UI.IMC_UI" 0 (struct)))

(event `self.Box.OnComponentBeginOverlap`
  (params (OverlappedComponent :type "PrimitiveComponent Object Reference") (OtherActor :type "Actor Object Reference") (OtherComp :type "PrimitiveComponent Object Reference") (OtherBodyIndex :type Integer) (bFromSweep :type Boolean) (SweepResult :type "HitResult Structure (by ref)"))
  (if (`self.ActorHasTag` OtherActor "Player")
    (`SceneComponent.SetHiddenInGame` (`self.Prompt`) false false)))

(event `self.Box.OnComponentEndOverlap`
  (params (OverlappedComponent :type "PrimitiveComponent Object Reference") (OtherActor :type "Actor Object Reference") (OtherComp :type "PrimitiveComponent Object Reference") (OtherBodyIndex :type Integer))
  (if (`self.ActorHasTag` OtherActor "Player")
    (`SceneComponent.SetHiddenInGame` (`self.Prompt`) true false)))

(fn `UserConstructionScript`)