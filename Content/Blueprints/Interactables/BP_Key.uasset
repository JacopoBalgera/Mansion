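; BP_Key is an interactable key pickup that adds to the interacting character's key count.
; OnInteraction calls CollectKey, which destroys the actor, then increments KeyCount on the passed character reference.
; Overlap events on the TextBox component show the TextRender when an overlap begins and hide it when it ends.
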(event `/Game/Blueprints/Interfaces/BPI_Interactions.OnInteraction`
  (params (CharacterReference :type "/Game/ThirdPerson/Blueprints/BP_ThirdPersonCharacter Object Reference"))
  ; OnInteraction
  (`self.CollectKey`)
  (`/Engine/EditorBlueprintResources/StandardMacros.IncrementInt` (`/Game/ThirdPerson/Blueprints/BP_ThirdPersonCharacter.KeyCount` CharacterReference)))

(event `CollectKey`
  ; KeyCollecting
  (`self.K2_DestroyActor`))

(event `self.TextBox.OnComponentBeginOverlap`
  (params (OverlappedComponent :type "PrimitiveComponent Object Reference") (OtherActor :type "Actor Object Reference") (OtherComp :type "PrimitiveComponent Object Reference") (OtherBodyIndex :type Integer) (bFromSweep :type Boolean) (SweepResult :type "HitResult Structure (by ref)"))
  (`SceneComponent.SetHiddenInGame` (`self.TextRender`) false false))

(event `self.TextBox.OnComponentEndOverlap`
  (params (OverlappedComponent :type "PrimitiveComponent Object Reference") (OtherActor :type "Actor Object Reference") (OtherComp :type "PrimitiveComponent Object Reference") (OtherBodyIndex :type Integer))
  (`SceneComponent.SetHiddenInGame` (`self.TextRender`) true false))

(fn `UserConstructionScript`)