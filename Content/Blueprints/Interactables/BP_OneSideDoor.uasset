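; Interactable hinged door that costs the interacting character a key the first time it opens, unless it is already unlocked.
; Interaction either decrements the character's key count and opens the door or shows the key dialogue when no key is held.
; A FlipFlop alternately plays and reverses a timeline that swings the door's yaw and sets it unlocked.
; Overlapping the TextBox component toggles two open/close prompts.
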(event `self.OnInteraction`
  (params (CharacterReference :type "/Game/ThirdPerson/Blueprints/BP_ThirdPersonCharacter Object Reference"))
  (bind _keycount (`/Game/ThirdPerson/Blueprints/BP_ThirdPersonCharacter.KeyCount` CharacterReference))
  ; OnInteraction
  (if (`self.IsUnlocked`)
    (`self.Open Door` :!label _label)
    (elif (> _keycount 0)
      (`/Engine/EditorBlueprintResources/StandardMacros.DecrementInt` _keycount
        (:`  `
          (goto _label)))
      (else
        (`/Game/ThirdPerson/Blueprints/BP_ThirdPersonCharacter.ShowKeyDialogue` CharacterReference)))))

(event `Open Door`
  ; Door system
  ;; Door opening
  (`/Engine/EditorBlueprintResources/StandardMacros.FlipFlop`
    (:`A`
      (bind (_direction _doorrotation) (`Timeline|OpenDoor Timeline` :!via `PlayFromStart` :!label _label_2)
        (:`Update`
          (`SceneComponent.K2_SetRelativeRotation` (`self.Door`) (`KismetMathLibrary.MakeRotator` 0.0 0.0 (`KismetMathLibrary.Lerp` 0.0 90.0 _doorrotation)) false false)
          (set `self.IsUnlocked` true))))
    (:`B`
      (goto _label_2 :!via `Reverse`))))

(event `self.TextBox.OnComponentBeginOverlap`
  (params (OverlappedComponent :type "PrimitiveComponent Object Reference") (OtherActor :type "Actor Object Reference") (OtherComp :type "PrimitiveComponent Object Reference") (OtherBodyIndex :type Integer) (bFromSweep :type Boolean) (SweepResult :type "HitResult Structure (by ref)"))
  ; PromptText
  (`SceneComponent.SetHiddenInGame` (`self.E to open/close`) false false)
  (`SceneComponent.SetHiddenInGame` (`self.E to open/close1`) false false))

(event `self.TextBox.OnComponentEndOverlap`
  (params (OverlappedComponent :type "PrimitiveComponent Object Reference") (OtherActor :type "Actor Object Reference") (OtherComp :type "PrimitiveComponent Object Reference") (OtherBodyIndex :type Integer))
  ; PromptText
  (`SceneComponent.SetHiddenInGame` (`self.E to open/close`) true false)
  (`SceneComponent.SetHiddenInGame` (`self.E to open/close1`) true false))

(fn `UserConstructionScript`)