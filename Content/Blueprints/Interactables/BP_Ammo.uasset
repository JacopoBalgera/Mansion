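; Interactable ammo pickup that adds its AmmoValue to the interacting character's ammo count.
; On BeginPlay it writes the value into a text render and caches the player controller.
; A box trigger shows its two text labels while an actor tagged Player overlaps it.
; OnInteraction adds the ammo, destroys the pickup and refreshes the ammo UI through the controller's Canvas.
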(event `self.ReceiveBeginPlay`
  (`|ExecutionSequence`
    (:`then_0`
      (`TextRenderComponent.K2_SetText` (`self.TextRender`) (`KismetTextLibrary.Conv_IntToText` (`self.AmmoValue`))))
    (:`then_1`
      (bind _asbp_player_controller (cast `/Game/ThirdPerson/Blueprints/BP_PlayerController` (`GameplayStatics.GetPlayerController` 0)))
      (set `self.ControllerRef` _asbp_player_controller))))

(event `self.Box.OnComponentBeginOverlap`
  (params (OverlappedComponent :type "PrimitiveComponent Object Reference") (OtherActor :type "Actor Object Reference") (OtherComp :type "PrimitiveComponent Object Reference") (OtherBodyIndex :type Integer) (bFromSweep :type Boolean) (SweepResult :type "HitResult Structure (by ref)"))
  (if (`self.ActorHasTag` OtherActor "Player")
    (`SceneComponent.SetHiddenInGame` (`self.TextRender`) false false)
    (`SceneComponent.SetHiddenInGame` (`self.AmmoText`) false false)))

(event `self.Box.OnComponentEndOverlap`
  (params (OverlappedComponent :type "PrimitiveComponent Object Reference") (OtherActor :type "Actor Object Reference") (OtherComp :type "PrimitiveComponent Object Reference") (OtherBodyIndex :type Integer))
  (if (`self.ActorHasTag` OtherActor "Player")
    (`SceneComponent.SetHiddenInGame` (`self.TextRender`) true false)
    (`SceneComponent.SetHiddenInGame` (`self.AmmoText`) true false)))

(event `/Game/Blueprints/Interfaces/BPI_Interactions.OnInteraction`
  (params (CharacterReference :type "/Game/ThirdPerson/Blueprints/BP_ThirdPersonCharacter Object Reference"))
  (set `/Game/ThirdPerson/Blueprints/BP_ThirdPersonCharacter.AmmoCount` (+ (`/Game/ThirdPerson/Blueprints/BP_ThirdPersonCharacter.AmmoCount` CharacterReference) (`self.AmmoValue`)) CharacterReference)
  (`self.K2_DestroyActor`)
  (`/Game/Blueprints/UI/WBP_Canvas.SetAmmoUI` (`/Game/ThirdPerson/Blueprints/BP_PlayerController.Canvas` (`self.ControllerRef`))))

(fn `UserConstructionScript`)