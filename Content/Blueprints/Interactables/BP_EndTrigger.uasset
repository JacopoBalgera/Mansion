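; BP_EndTrigger is a box trigger that runs the game's ending sequence when an actor tagged Player overlaps it.
; It removes the default input mapping, stops the camera boom following control rotation and pulls the camera back on a timeline.
; It also unhides BP_Kendrick and lets him move.
; Delays then play a Kendrick text fade on the controller's canvas and open the end menu with UI-only input and, later, the mouse cursor.
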(event `self.ReceiveBeginPlay`
  (`|ExecutionSequence`
    (:`then_0`
      (bind _asbp_player_controller (cast `/Game/ThirdPerson/Blueprints/BP_PlayerController` (`GameplayStatics.GetPlayerController` 0)))
      (set `self.ControllerRef` _asbp_player_controller))
    (:`then_1`
      (bind _asbp_third_person_character (cast `/Game/ThirdPerson/Blueprints/BP_ThirdPersonCharacter` (`GameplayStatics.GetPlayerCharacter` 0)))
      (set `self.PlayerRef` _asbp_third_person_character))))

(event `self.Box.OnComponentBeginOverlap`
  (params (OverlappedComponent :type "PrimitiveComponent Object Reference") (OtherActor :type "Actor Object Reference") (OtherComp :type "PrimitiveComponent Object Reference") (OtherBodyIndex :type Integer) (bFromSweep :type Boolean) (SweepResult :type "HitResult Structure (by ref)"))
  (bind _returnvalue (`GameplayStatics.GetPlayerController` 0))
  (bind _playerref (`self.PlayerRef`))
  (bind _canvas (`/Game/ThirdPerson/Blueprints/BP_PlayerController.Canvas` (`self.ControllerRef`)))
  (bind _cameraboom (`/Game/ThirdPerson/Blueprints/BP_ThirdPersonCharacter.CameraBoom` _playerref))
  (if (`self.ActorHasTag` OtherActor "Player")
    (`|ExecutionSequence`
      (:`then_0`
        (`EnhancedInputSubsystemInterface.RemoveMappingContext` (pcsubsystem `EnhancedInputLocalPlayerSubsystem` (`self.ControllerRef`)) "/Game/ThirdPerson/Input/IMC_Default.IMC_Default" (struct)))
      (:`then_1`
        (set `SpringArmComponent.bUsePawnControlRotation` false _cameraboom)
        (`SceneComponent.K2_SetRelativeRotation` :`self` (`/Game/ThirdPerson/Blueprints/BP_ThirdPersonCharacter.FollowCamera` _playerref))
        (bind (_direction _newtrack_0) (`Timeline|CameraDistance` :!via `PlayFromStart`)
          (:`Update`
            (set `SpringArmComponent.TargetArmLength` (`KismetMathLibrary.Lerp` 200.0 300.0 _newtrack_0) _cameraboom))))
      (:`then_2`
        (bind _returnvalue_2 (`GameplayStatics.GetActorOfClass` "/Game/Blueprints/IA/BP_Kendrick.BP_Kendrick_C"))
        (set `/Game/Blueprints/IA/BP_Kendrick.CanMove` true _returnvalue_2)
        (`SceneComponent.SetHiddenInGame` (`Character.Mesh` _returnvalue_2) false false))
      (:`then_3`
        (`KismetSystemLibrary.Delay` 3.0)
        (`UserWidget.PlayAnimation` _canvas (`/Game/Blueprints/UI/BP_Canvas.TextFadeKendrick` _canvas) 0.0 1 "Forward" 1.0 false))
      (:`then_4`
        (`KismetSystemLibrary.Delay` 7.0)
        (bind _returnvalue_3 (`|CreateWidget` "/Game/Blueprints/UI/BP_EndMenu.BP_EndMenu_C" _returnvalue))
        (`UserWidget.AddToViewport` _returnvalue_3 0)
        (`WidgetBlueprintLibrary.SetInputMode_UIOnlyEx` _returnvalue _returnvalue_3)
        (`KismetSystemLibrary.Delay` 2.0)
        (set `PlayerController.bShowMouseCursor` true _returnvalue)))))

(fn `UserConstructionScript`)