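; BP_DialogueTrigger is an overlap trigger actor that starts a dialogue text fade on the player's UI.
; On BeginPlay it caches the first player controller, cast to BP_PlayerController.
; When the player character overlaps it, it plays the TextFadeStartingDialogue animation on that controller's Canvas widget, with no guard against repeat triggering.
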(event `self.ReceiveBeginPlay`
  (bind _asbp_player_controller (cast `/Game/ThirdPerson/Blueprints/BP_PlayerController` (`GameplayStatics.GetPlayerController` 0)))
  (set `self.ControllerRef` _asbp_player_controller))

(event `self.ReceiveActorBeginOverlap`
  (params (OtherActor :type "Actor Object Reference"))
  (bind _canvas (`/Game/ThirdPerson/Blueprints/BP_PlayerController.Canvas` (`self.ControllerRef`)))
  (if (== OtherActor (`GameplayStatics.GetPlayerCharacter` 0))
    (`UserWidget.PlayAnimation` _canvas (`/Game/Blueprints/UI/WBP_Canvas.TextFadeStartingDialogue` _canvas) 0.0 1 "Forward" 1.0 false)))

(fn `UserConstructionScript`)